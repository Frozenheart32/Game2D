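; BP_Skeleton is a skeleton enemy character that paces back and forth along the X axis and damages actors touching its hit box.
; Despite its name, Follow tracks no target: each Tick it moves and steps a counter toward a limit, then negates the limit and rotates the sprite.
; A BoxHit overlap applies damage, launches the skeleton itself along +X, and briefly locks its movement.
; Patrol distance depends on frame rate because the counter advances per tick.
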(event `self.ReceiveTick`
  (params (DeltaSeconds :type "Float (single-precision)"))
  (`self.Follow`))

(event `self.BoxHit.OnComponentBeginOverlap`
  (params (OverlappedComponent :type "PrimitiveComponent Object Reference") (OtherActor :type "Actor Object Reference") (OtherComp :type "PrimitiveComponent Object Reference") (OtherBodyIndex :type Integer) (bFromSweep :type Boolean) (SweepResult :type "HitResult Structure (by ref)"))
  (`GameplayStatics.ApplyDamage` OtherActor 10.0)
  (`self.LaunchCharacter` (500.0 0.0 0.0) true)
  (set `self.IsMovementLock` true)
  (`KismetSystemLibrary.Delay` 2.0)
  (set `self.IsMovementLock` false))

(event `Follow`
  (bind _sprite (`self.Sprite`))
  (if (not (`self.IsMovementLock`))
    (`/Engine/EditorBlueprintResources/StandardMacros.CompareFloat` (`self.S1`) (`self.S`)
      (:`>`
        (`self.AddMovementInput` (-1.0 0.0 0.0))
        (`/Engine/EditorBlueprintResources/StandardMacros.DecrementFloat` (`self.S1`)))
      (:`==`
        (set `self.S` (* (`self.S`) -1.0))
        (set `self.S1` 0.0)
        (if (> (`self.S`) 0.0)
          (`SceneComponent.K2_SetRelativeRotation` _sprite (struct :`Yaw` 180.0) false false)
          (else
            (`SceneComponent.K2_SetRelativeRotation` _sprite (struct) false false))))
      (:`<`
        (`self.AddMovementInput` (1.0 0.0 0.0))
        (`/Engine/EditorBlueprintResources/StandardMacros.IncrementFloat` (`self.S1`))))))

(fn `UserConstructionScript`)